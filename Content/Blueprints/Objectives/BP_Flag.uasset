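; Flag objective actor whose skeletal-mesh flag rises and falls with an inherited Status value, lerped into its height every tick.
; The construction script applies a configurable collision mesh, whose begin-overlap event calls Update.
; DetermineTeam tallies overlapping actors by their team message, reporting whether team 1 or 2 is present.
; Its TeamID output carries the larger of those two tallies rather than a team index.
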(event `self.ReceiveTick`
  (params (DeltaSeconds :type "Float (single-precision)"))
  (`parent.ReceiveTick` DeltaSeconds)
  (`self.MoveFlag` (`self.Status`)))

(event `self.CollisionMeshContainer.OnComponentBeginOverlap`
  (params (OverlappedComponent :type "PrimitiveComponent Object Reference") (OtherActor :type "Actor Object Reference") (OtherComp :type "PrimitiveComponent Object Reference") (OtherBodyIndex :type Integer) (bFromSweep :type Boolean) (SweepResult :type "HitResult Structure (by ref)"))
  (`self.Update`))

(fn `DetermineTeam`
  (returns (TeamID :type Integer) (bHasAnyone :type Boolean))
  (locals (TeamReference :type "Array of Integer"))
  (bind _teamreference (`local.TeamReference`))
  (bind _output (`|GetArrayItem` _teamreference 2))
  (bind _output_2 (`|GetArrayItem` _teamreference 1))
  (`parent.DetermineTeam`)
  (for _array_element (`PrimitiveComponent.GetOverlappingActors` (`self.CollisionMeshContainer`) "/Script/Engine.Actor")
    (bind _team (message `/Game/Blueprints/Interfaces/BPI_Teams.GetTeam` _array_element))
    (`/Engine/EditorBlueprintResources/StandardMacros.IncrementInt` (`|GetArrayItem` (`local.TeamReference`) _team)))
  (return (select `bool` (> _output_2 _output) :`false` _output :`true` _output_2) (or (> _output_2 0) (> _output 0))))

(fn `MoveFlag`
  (params (t :type "Float (double-precision)"))
  (bind (_relativelocation_x _relativelocation_y) (`KismetMathLibrary.BreakVector` (`SceneComponent.RelativeLocation` (`self.SkeletalMesh`))))
  (`SceneComponent.K2_SetRelativeLocation` (`self.SkeletalMesh`) (`KismetMathLibrary.MakeVector` _relativelocation_x _relativelocation_y (`KismetMathLibrary.Lerp` 120.0 710.0 t)) false false)
  (`SceneComponent.K2_SetRelativeLocation` (`self.SkeletalMesh`) (`KismetMathLibrary.MakeVector` _relativelocation_x _relativelocation_y (`KismetMathLibrary.Lerp` 120.0 710.0 t)) false false))

(fn `UserConstructionScript`
  (`parent.UserConstructionScript`)
  (`StaticMeshComponent.SetStaticMesh` (`self.CollisionMeshContainer`) (`self.CollisionMesh`)))