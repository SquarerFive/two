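; Base capturable objective actor that tracks an owning team and capture progress, leaving DetermineTeam as a stub for child classes.
; Update runs a Capture timeline forward when neutral or backward when another team must neutralize the owner, stopping if the owner's team returns.
; Timeline alpha drives Status, and completion sets Team to the capturer or neutral.
; Construction derives play rate from CaptureSpeed; Team and Name have empty RepNotify handlers.
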(event `Update`
  (bind _team (`self.Team`))
  (bind _teamid (`self.DetermineTeam`))
  (if (!= _teamid _team)
    (if (!= _team 0)
      (bind (_direction _alpha) (`Timeline|Capture` :!via `Reverse` :!label _label)
        (:`Update`
          (bind _teamid_2 (`self.DetermineTeam`))
          (if (== (`self.Team`) _teamid_2)
            (goto _label :!via `Stop`)
            (else
              (set `self.Status` _alpha))))
        (:`Finished`
          (switch `ETimelineDirection` _direction
            (:`Forward`
              (bind _teamid_3 (`self.DetermineTeam`))
              (set `self.Team` _teamid_3))
            (:`Backward`
              (set `self.Team` 0)))))
      (else
        (goto _label)))))

(fn `DetermineTeam`
  (returns (TeamID :type Integer) (bHasAnyone :type Boolean))
  ;[1 1 1] This will be overidden by child classes.
  (return 0 false))

(fn `OnRep_Name`)

(fn `OnRep_Team`)

(fn `UserConstructionScript`
  (`TimelineComponent.SetPlayRate` (`self.Capture`) (/ 1.0 (`self.CaptureSpeed`))))