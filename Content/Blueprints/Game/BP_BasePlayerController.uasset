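; BP_BasePlayerController is a player controller that spawns and possesses a ThirdPersonCharacter at an objective.
; Spawn checks authority, running the spawn logic directly on the server or calling ServerSpawn from a client.
; The logic places the character slightly above the first BP_BaseObjective found, always spawning regardless of collision, then possesses it.
; Random-point-in-bounds placement nodes remain in the graph but are unused.
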(event `Server Spawn`
  (bind _outactors (`GameplayStatics.GetAllActorsOfClass` "/Game/Blueprints/Objectives/BP_BaseObjective.BP_BaseObjective_C" :!label _label))
  (bind (_returnvalue_x _returnvalue_y _returnvalue_z) (`KismetMathLibrary.BreakVector` (`self.K2_GetActorLocation` (`|GetArrayItem` _outactors))))
  (bind _returnvalue (`|SpawnActorFromClass` "/Game/ThirdPersonBP/Blueprints/ThirdPersonCharacter.ThirdPersonCharacter_C" (`KismetMathLibrary.Conv_VectorToTransform` (`KismetMathLibrary.MakeVector` _returnvalue_x _returnvalue_y (+ _returnvalue_z 100.0))) "AlwaysSpawn" "OverrideRootScale" null null))
  (`self.Possess` _returnvalue))

(event `/Game/Blueprints/Interfaces/BPI_Player.Spawn`
  (`/Engine/EditorBlueprintResources/ActorMacros.Switch Has Authority`
    (:`Authority`
      (goto _label))
    (:`Remote`
      (`self.Server Spawn`))))

(fn `UserConstructionScript`)