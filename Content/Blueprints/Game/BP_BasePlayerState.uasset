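; BP_BasePlayerState is a player state Blueprint that holds the player's Team and keeps objective colours and the minimap matched to it.
; On BeginPlay it finds the first BP_MinimapManager, binds to its NotifyUpdate dispatcher and runs that update handler once.
; Each update passes Team to every BP_BaseObjective to update its colours, then tells the minimap manager to render.
; GetTeam exposes the Team value.
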(event `self.ReceiveBeginPlay`
  (bind _outactors (`GameplayStatics.GetAllActorsOfClass` "/Game/Blueprints/Minimap/BP_MinimapManager.BP_MinimapManager_C"))
  (bind _output_get (set `self.MinimapManager` (`|GetArrayItem` _outactors)))
  (add `/Game/Blueprints/Minimap/BP_MinimapManager.Notify Update` _output_get (delegate `Notify Update_Event_0`))
  (`self.Notify Update_Event_0`))

(event `Notify Update_Event_0`
  (bind _outactors (`GameplayStatics.GetAllActorsOfClass` "/Game/Blueprints/Objectives/BP_BaseObjective.BP_BaseObjective_C"))
  (for _array_element _outactors
    (`/Game/Blueprints/Objectives/BP_BaseObjective.UpdateColours` _array_element (`self.Team`)))
  (`/Game/Blueprints/Minimap/BP_MinimapManager.Render` (`self.MinimapManager`)))

(fn `GetTeam`
  (returns (Team :type Integer))
  (return (`self.Team`)))

(fn `UserConstructionScript`)