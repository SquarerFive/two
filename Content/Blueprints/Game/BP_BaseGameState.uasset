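; Base game state that runs a team ticket bleed driven by objective ownership.
; On the server, BeginPlay starts a five-second looping timer and copies the match start time from BP_BaseGameMode.
; Each tick of that timer counts cached BP_BaseObjective actors per team and decrements tickets of the team holding fewer, or index 0 on a tie.
; BroadcastTicketUpdate then fires the OnTicketsUpdate dispatcher; OnRep_Tickets is empty.
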(event `self.ReceiveBeginPlay`
  (`/Engine/EditorBlueprintResources/ActorMacros.Switch Has Authority`
    (:`Authority`
      (`KismetSystemLibrary.K2_SetTimerDelegate` (delegate `Timer Tickets`) 5.0 true)
      (bind _asbp_base_game_mode (cast `/Game/Blueprints/Game/BP_BaseGameMode` (`GameplayStatics.GetGameMode`)))
      (set `self.MatchStart` (`/Game/Blueprints/Game/BP_BaseGameMode.MatchStartTime` _asbp_base_game_mode)))))

(event `Timer Tickets`
  (`self.Update Tickets`))

(event `Broadcast Ticket Update`
  (`self.OnTicketsUpdate`))

(fn `OnRep_Tickets`)

(fn `Update Tickets`
  (locals (TeamCount :type "Array of Integer"))
  (bind _teamcount (`local.TeamCount`))
  (bind _output (`|GetArrayItem` _teamcount 2))
  (bind _output_2 (`|GetArrayItem` _teamcount 1))
  (if (not (> (`KismetArrayLibrary.Array_Length` (`self.Objectives`)) 0))
    (bind _outactors (`GameplayStatics.GetAllActorsOfClass` "/Game/Blueprints/Objectives/BP_BaseObjective.BP_BaseObjective_C"))
    (set `self.Objectives` _outactors))
  (for _array_element (`self.Objectives`)
    (`/Engine/EditorBlueprintResources/StandardMacros.IncrementInt` (`|GetArrayItem` _teamcount (`/Game/Blueprints/Objectives/BP_BaseObjective.Team` _array_element))))
  (`/Engine/EditorBlueprintResources/StandardMacros.DecrementInt` (`|GetArrayItem` (`self.Tickets`) (select `bool` (> _output_2 _output) :`false` (select `bool` (> _output _output_2) :`true` 1) :`true` 2))
    (:`  `
      (`self.Broadcast Ticket Update`))))

(fn `UserConstructionScript`)