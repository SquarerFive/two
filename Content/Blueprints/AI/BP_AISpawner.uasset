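; BP_AISpawner populates an area with ThirdPersonCharacter instances when play begins.
; On the authority only, BeginPlay calls Spawn, which creates MaxAI characters at random points inside the Box component's bounds.
; Spawns adjust for collisions but always succeed, and each character is randomly assigned to team 1 or 2.
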(event `self.ReceiveBeginPlay`
  (`/Engine/EditorBlueprintResources/ActorMacros.Switch Has Authority`
    (:`Authority`
      (`self.Spawn`))))

(event `Spawn`
  (bind _box (`self.Box`))
  (for _ (range (`self.MaxAI`))
    (bind _returnvalue (`|SpawnActorFromClass` "/Game/ThirdPersonBP/Blueprints/ThirdPersonCharacter.ThirdPersonCharacter_C" (`KismetMathLibrary.Conv_VectorToTransform` (`KismetMathLibrary.RandomPointInBoundingBox` (`SceneComponent.K2_GetComponentLocation` _box) (`BoxComponent.BoxExtent` _box))) "AdjustIfPossibleButAlwaysSpawn" "OverrideRootScale" null null))
    (`/Game/ThirdPersonBP/Blueprints/ThirdPersonCharacter.Set Team` _returnvalue (select `bool` (`KismetMathLibrary.RandomBool`) :`false` 1 :`true` 2))))

(fn `UserConstructionScript`)