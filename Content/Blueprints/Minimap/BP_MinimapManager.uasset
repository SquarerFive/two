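; BP_MinimapManager is a minimap actor that captures the level through an orthographic scene capture component.
; Setup, run from the construction script, applies the Width value to both the camera and the scene capture.
; SetWidthFromActorBounds derives Width from the length of a referenced actor's XY bounds extent, then reruns Setup.
; Capture happens on demand through the Render event, with no active Tick or BeginPlay logic.
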(event `Render`
  (`SceneCaptureComponent2D.CaptureScene` (`self.SceneCaptureComponent2D`)))

(event `SetWidthFromActorBounds`
  (set `self.Width` (`KismetMathLibrary.VSize2D` (`KismetMathLibrary.MakeVector2D` (.x (`.BoxExtent` (`self.GetActorBounds` (`self.Actor`) false))) (.y (`.BoxExtent` (`self.GetActorBounds` (`self.Actor`) false))))))
  (`self.Setup`))

(fn `Setup`
  (bind _width (`self.Width`))
  (bind _scenecapturecomponent2d (`self.SceneCaptureComponent2D`))
  (`CameraComponent.SetOrthoWidth` (`self.Camera`) _width)
  (set `SceneCaptureComponent2D.OrthoWidth` _width _scenecapturecomponent2d)
  (set `SceneCaptureComponent2D.ProjectionType` "Orthographic" _scenecapturecomponent2d))

(fn `UserConstructionScript`
  (`self.Setup`))